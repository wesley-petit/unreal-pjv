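; BP_Swim_Area is a trigger actor that marks a swimming zone for the third-person character.
; When a BP_ThirdPersonCharacter_2 begins overlapping it, it sets InWater to true on that character's ABP_Mixamo animation instance, and clears the flag when the overlap ends.
; It only drives the animation flag; movement mode and physics are not changed here.
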(event `self.ReceiveActorBeginOverlap`
  (params (OtherActor :type "Actor Object Reference"))
  (bind _asbp_third_person_character_2 (cast `/Game/CreationEvaluation/Nage/BP_ThirdPersonCharacter_2` OtherActor))
  (bind _asabp_mixamo (cast `/Game/CreationEvaluation/Nage/Character/Animations/ABP_Mixamo` (`SkeletalMeshComponent.GetAnimInstance` (`Character.Mesh` _asbp_third_person_character_2))))
  (set `/Game/CreationEvaluation/Nage/Character/Animations/ABP_Mixamo.bInWater` true _asabp_mixamo))

(event `self.ReceiveActorEndOverlap`
  (params (OtherActor :type "Actor Object Reference"))
  (bind _asbp_third_person_character_2 (cast `/Game/CreationEvaluation/Nage/BP_ThirdPersonCharacter_2` OtherActor))
  (bind _asabp_mixamo (cast `/Game/CreationEvaluation/Nage/Character/Animations/ABP_Mixamo` (`SkeletalMeshComponent.GetAnimInstance` (`Character.Mesh` _asbp_third_person_character_2))))
  (set `/Game/CreationEvaluation/Nage/Character/Animations/ABP_Mixamo.bInWater` false _asabp_mixamo))

(fn `UserConstructionScript`)