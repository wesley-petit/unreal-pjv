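; BP_CoinStand is a creation piece that switches coin rotation along with its functionality state.
; On BeginPlay it caches every BP_BasicCoin actor in the level, not just coins tied to this stand.
; Its ShowFunctionality and HideFunctionality overrides call the parent, then turn rotation on or off for each cached coin, printing a debug string per coin.
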(event `self.ReceiveBeginPlay`
  (`parent.ReceiveBeginPlay`)
  (bind _outactors (`GameplayStatics.GetAllActorsOfClass` "/Game/CreationEvaluation/Pieces/BP_BasicCoin.BP_BasicCoin_C"))
  (set `self.Coins` _outactors))

(fn `HideFunctionality`
  (`parent.HideFunctionality`)
  (for _array_element (`self.Coins`)
    (`/Game/CreationEvaluation/Pieces/BP_BasicCoin.ChangeRotateState` _array_element false)
    (`KismetSystemLibrary.PrintString` "Hide")))

(fn `ShowFunctionality`
  (`parent.ShowFunctionality`)
  (for _array_element (`self.Coins`)
    (`/Game/CreationEvaluation/Pieces/BP_BasicCoin.ChangeRotateState` _array_element true)
    (`KismetSystemLibrary.PrintString` "Show")))

(fn `UserConstructionScript`
  (`parent.UserConstructionScript`))